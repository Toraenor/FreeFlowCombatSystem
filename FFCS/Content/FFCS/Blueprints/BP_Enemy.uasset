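; BP_Enemy is an enemy character that reacts to hits and ragdolls when its health runs out.
; On AnyDamage, ACEnemyComp resolves the hit direction from the damage causer to pick one of four directional hit montages.
; Each hit removes one health point regardless of damage amount and prints the remaining health.
; At zero, it disables movement and capsule collision, enables mesh physics and marks ACEnemyComp as untargetable.
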(event Game|Damage|EventAnyDamage
  (params (Damage :type Float%20%28single-precision%29) (DamageType :type Damage%20Type%20Object%20Reference) (InstigatedBy :type Controller%20Object%20Reference) (DamageCauser :type Actor%20Object%20Reference))
  (Animation|Montage|PlayMontage (Variables|Character|GetMesh) (Utilities|Select :Index (Default|GetHitDirection (Variables|Default|GetAC_EnemyComp) DamageCauser) :NewEnumerator0 "/Game/FFCS/Animations/AnimMontages/AM_HitFromForward.AM_HitFromForward" :NewEnumerator1 "/Game/FFCS/Animations/AnimMontages/AM_HitFromRight.AM_HitFromRight" :NewEnumerator2 "/Game/FFCS/Animations/AnimMontages/AM_HitFromBackward.AM_HitFromBackward" :NewEnumerator3 "/Game/FFCS/Animations/AnimMontages/AM_HitFromLeft.AM_HitFromLeft")
    (:then
      (bind _output_get (Variables|Default|SetCurrentHealth (Math|Float|Clamp(Float) (- (Variables|Default|GetCurrentHealth) 1.0) 0.0 (Variables|Default|GetMaxHealth))))
      (Development|PrintString (Utilities|String|ToString(Float) _output_get) true true "(R=0.000000,G=1.000000,B=0.030613,A=1.000000)")
      (if (== (Variables|Default|GetCurrentHealth) 0.0)
        (Pawn|Components|CharacterMovement|SetMovementMode (Variables|Character|GetCharacterMovement) "MOVE_None" 0)
        (Physics|SetSimulatePhysics (Variables|Character|GetMesh) true)
        (Collision|SetCollisionEnabled (Variables|Default|GetCapsuleComponent) "NoCollision")
        (Collision|SetCollisionEnabled (Variables|Character|GetMesh) "QueryAndPhysics")
        (Variables|/Game/FFCS/Blueprints/AC_EnemyComp.AC_EnemyComp_C|SetTargetable (Variables|Default|GetAC_EnemyComp) false)))))

(fn ConstructionScript
  (|CallParentFunction))