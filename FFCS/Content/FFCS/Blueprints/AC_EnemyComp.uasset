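; Enemy component that works out which side its owner is hit from, relative to the owner's facing.
; GetHitDirection takes the yaw delta between the look-at rotation toward the instigator and the owner's rotation.
; It sorts that yaw into forward, right, backward or left quadrants and returns an enum, splitting the backward range across the ±180° wrap.
; The event graph has no active logic.
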(event EventBeginPlay)

(event EventTick
  (params (DeltaSeconds :type Float%20%28single-precision%29)))

(fn GetHitDirection
  (params (Instigator :type Actor%20Object%20Reference))
  (bind _returnvalue (Transformation|GetActorLocation Instigator))
  (bind _returnvalue_2 (Components|GetOwner))
  (bind _returnvalue_3 (Transformation|GetActorRotation _returnvalue_2))
  (bind _returnvalue_4 (Transformation|GetActorLocation _returnvalue_2))
  (bind _returnvalue_5 (Math|Rotator|FindLookatRotation _returnvalue_4 _returnvalue))
  (bind _returnvalue_6 (Math|Rotator|Delta(Rotator) _returnvalue_5 _returnvalue_3))
  ;[1 0.1521 0.8232] Checking from direction enemy has been hit, in order :
  ; Forward
  ; Right
  ; Backward
  ; Left
  (if (Math|Float|InRange(Float) (.yaw _returnvalue_6) -45.0 45.0)
    (return "NewEnumerator0")
    (elif (Math|Float|InRange(Float) (.yaw _returnvalue_6) 45.0 135.0)
      (return "NewEnumerator1")
      (elif (or (Math|Float|InRange(Float) (.yaw _returnvalue_6) 135.0 1.8e+02) (Math|Float|InRange(Float) (.yaw _returnvalue_6) -179.99 -135.0))
        (return "NewEnumerator2")
        (else
          (return "NewEnumerator3"))))))