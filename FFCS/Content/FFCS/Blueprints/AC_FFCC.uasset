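; AC_FFCC is a combat-state component that stores the current enemy and the player's state gameplay tag.
; Simple setters and getters expose both values, and setting the tag also prints its name for debugging.
; IsEnemyAlreadyHit both checks and records: it adds unseen enemies to a list and returns false, or true for repeats.
; Nothing here clears that list, and BeginPlay and Tick are unused.
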(event EventBeginPlay)

(event EventTick
  (params (DeltaSeconds :type Float%20%28single-precision%29)))

(fn SetCurrentEnemy
  (params (CurrentEnemy :type Actor%20Object%20Reference))
  (Variables|Default|SetCurrentEnemy CurrentEnemy))

(fn GetCurrentEnemy
  (return (Variables|Default|GetCurrentEnemy)))

(fn SetTagtoPlayer
  (params (Tag :type Gameplay%20Tag%20Structure))
  (bind _output_get (Variables|Default|SetPlayerStateTag Tag))
  (Development|PrintString (Utilities|String|ToString(Name) (GameplayTags|GetTagName _output_get))))

(fn GetPlayerTag
  (return (Variables|Default|GetPlayerStateTag)))

(fn IsEnemyAlreadyHit
  (params (Enemy :type Actor%20Object%20Reference))
  (if (Utilities|Array|ContainsItem (Variables|Default|GetEnemiesAlreadyHit) Enemy)
    (return true)
    (else
      (Utilities|Array|Add (Variables|Default|GetEnemiesAlreadyHit) Enemy)
      (return false))))