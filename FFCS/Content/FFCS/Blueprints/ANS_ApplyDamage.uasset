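; Anim notify state that opens a melee damage window during attack animations in the FFCS combat system.
; On begin it sets the owner's AC_FFCC state to CombatInProgress; each tick it sphere-traces along the right-hand weapon bones.
; Characters not already hit take damage and raise the owner's combo.
; On end it restores Combat state, resets the combo if nothing was hit, and clears the hit list.
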(fn ReceivedNotifyBegin
  (params (MeshComp :type Skeletal%20Mesh%20Component%20Object%20Reference) (Animation :type Anim%20Sequence%20Base%20Object%20Reference) (TotalDuration :type Float%20%28single-precision%29) (EventReference :type Anim%20Notify%20Event%20Reference%20Structure%20%28by%20ref%29))
  (bind _returnvalue (Components|GetOwner MeshComp))
  (bind _returnvalue_2 (Actor|GetComponentbyClass _returnvalue "/Game/FFCS/Blueprints/AC_FFCC.AC_FFCC_C"))
  (Utilities|IsValid _returnvalue_2
    (:Is%20Valid
      (Default|SetTagtoPlayer _returnvalue_2 "(TagName=\"PlayerStates.CombatInProgress\")")
      (return true))))

(fn ReceivedNotifyTick
  (params (MeshComp :type Skeletal%20Mesh%20Component%20Object%20Reference) (Animation :type Anim%20Sequence%20Base%20Object%20Reference) (FrameDeltaTime :type Float%20%28single-precision%29) (EventReference :type Anim%20Notify%20Event%20Reference%20Structure%20%28by%20ref%29))
  (bind _returnvalue (Components|GetOwner MeshComp))
  (bind _debugbool (Class|BPIDebugKeys|GetDebugBool(Message) (Game|GetPlayerController MeshComp)))
  (bind _outhits (Collision|MultiSphereTraceByChannel MeshComp (.location (Transformation|GetBoneTransform MeshComp "Weapon_R" "RTS_World")) (.location (Transformation|GetBoneTransform MeshComp "Weapon_R_Muzzle" "RTS_World")) 2e+01 "TraceTypeQuery1" false 0 (select _debugbool "ForDuration" "None")))
  (for _array_element _outhits
    (if (Class|GameplayStatics|ObjectIsA (.hitactor _array_element) "/Game/FFCS/Blueprints/BP_CharacterBase.BP_CharacterBase_C")
      (bind _output_get (LocalVariables|SetCurrentEnemy (.hitactor _array_element)))
      (bind _isenemyhit (Default|IsEnemyAlreadyHit (Actor|GetComponentbyClass (Components|GetOwner MeshComp) "/Game/FFCS/Blueprints/AC_FFCC.AC_FFCC_C") _output_get))
      (if (not _isenemyhit)
        (Game|Damage|ApplyDamage (LocalVariables|GetCurrentEnemy) 1.0 0 _returnvalue "/Script/Engine.DamageType")
        (Class|BPIPlayer|IncreaseCombo(Message) _returnvalue))))
  (return true))

(fn ReceivedNotifyEnd
  (params (MeshComp :type Skeletal%20Mesh%20Component%20Object%20Reference) (Animation :type Anim%20Sequence%20Base%20Object%20Reference) (EventReference :type Anim%20Notify%20Event%20Reference%20Structure%20%28by%20ref%29))
  (bind _returnvalue (Components|GetOwner MeshComp))
  (bind _returnvalue_2 (Actor|GetComponentbyClass _returnvalue "/Game/FFCS/Blueprints/AC_FFCC.AC_FFCC_C"))
  (bind _enemiesalreadyhit (Variables|/Game/FFCS/Blueprints/AC_FFCC.AC_FFCC_C|GetEnemiesAlreadyHit _returnvalue_2))
  (Utilities|IsValid _returnvalue_2
    (:Is%20Valid
      (Default|SetTagtoPlayer _returnvalue_2 "(TagName=\"PlayerStates.Combat\")")
      (if (== (Utilities|Array|Length _enemiesalreadyhit) 0)
        (Class|BPIPlayer|ResetCombo(Message) (Components|GetOwner MeshComp)))
      (Utilities|Array|Clear _enemiesalreadyhit)
      (return true))))