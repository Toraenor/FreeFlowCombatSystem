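; AI director component that tracks enemies in a fight and coordinates which one attacks the player.
; AddEnemy registers unique enemies, signals fight entry on the first, and starts a looping timer with a randomized period, cleared when RemoveEnemy empties the list.
; CheckIfPlayerUnderAttack flags a random enemy to attack through AC_EnemyComp when none is attacking, respecting stopped logic.
; ToggleAllEnemiesLogic switches logic across all registered enemies.
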(event EventBeginPlay)

(event EventTick
  (params (DeltaSeconds :type Float%20%28single-precision%29)))

(fn AddEnemy
  (params (Enemy :type Actor%20Object%20Reference))
  (bind _returnvalue (Utilities|Array|AddUnique (Variables|Default|GetEnemies) Enemy))
  (if (== 0 _returnvalue)
    (Default|CallEnterFight))
  (if (and (> (Utilities|Array|Length (Variables|Default|GetEnemies)) 0) (not (Utilities|Time|IsTimerActivebyHandle (Variables|Default|GetCheckAttackPlayerTH))))
    (bind _returnvalue_2 (Utilities|Time|SetTimerbyEvent (EventDispatchers|CreateEvent :!event CheckifPlayerUnderAttack) (Math|Random|RandomFloatinRange 0.5 2.0) true true))
    (Variables|Default|SetCheckAttackPlayerTH _returnvalue_2)))

(fn CheckifPlayerUnderAttack
  (bind _enemies (Variables|Default|GetEnemies))
  (bind _outitem (Utilities|Array|Random _enemies))
  (bind _returnvalue (Actor|GetComponentbyClass _outitem "/Game/FFCS/Blueprints/AC_EnemyComp.AC_EnemyComp_C"))
  (LocalVariables|SetChooseAIToAttack true)
  (for _array_element (Variables|Default|GetEnemies)
    (Utilities|IsValid (Actor|GetComponentbyClass _array_element "/Game/FFCS/Blueprints/AC_EnemyComp.AC_EnemyComp_C")
      (:Is%20Valid
        (if (Default|GetAttackPlayer (Actor|GetComponentbyClass _array_element "/Game/FFCS/Blueprints/AC_EnemyComp.AC_EnemyComp_C"))
          (LocalVariables|SetChooseAIToAttack false)))))
  (if (LocalVariables|GetChooseAIToAttack)
    (Utilities|IsValid _returnvalue
      (:Is%20Valid
        (if (not (Variables|/Game/FFCS/Blueprints/AC_EnemyComp.AC_EnemyComp_C|GetLogicStopped _returnvalue))
          (Default|SetAttackPlayer _returnvalue true))))))

(fn RemoveEnemy
  (params (Enemy :type Actor%20Object%20Reference))
  (Utilities|Array|RemoveItem (Variables|Default|GetEnemies) Enemy)
  (if (<= (Utilities|Array|Length (Variables|Default|GetEnemies)) 0)
    (Utilities|Time|ClearandInvalidateTimerbyHandle (Variables|Default|GetCheckAttackPlayerTH))))

(fn ToggleAllEnemiesLogic
  (params (Disable :type Boolean))
  (for _array_element (Variables|Default|GetEnemies)
    (Default|ControlEnemyLogic (Actor|GetComponentbyClass _array_element "/Game/FFCS/Blueprints/AC_EnemyComp.AC_EnemyComp_C") Disable)))