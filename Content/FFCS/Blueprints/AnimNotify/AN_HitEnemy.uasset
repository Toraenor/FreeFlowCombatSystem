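; Anim notify that lands a melee hit on the owner's current enemy from AC_FFCC, dealing 1 damage and incrementing the combo message.
; Before damage, it plays a camera shake if the target has 1 health and is the last enemy in AC_AIDirector.
; That check reads the current enemy in the Combat state and the counter enemy otherwise, though damage always goes to the current enemy.
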(fn ReceivedNotify
  (params (MeshComp :type Skeletal%20Mesh%20Component%20Object%20Reference) (Animation :type Anim%20Sequence%20Base%20Object%20Reference) (EventReference :type Anim%20Notify%20Event%20Reference%20Structure%20%28by%20ref%29))
  (bind _returnvalue (Components|GetOwner MeshComp))
  (bind _returnvalue_2 (Actor|GetComponentbyClass _returnvalue "/Game/FFCS/Blueprints/AC_FFCC.AC_FFCC_C"))
  (bind _returnvalue_3 (Default|GetCurrentEnemy _returnvalue_2))
  (Utilities|IsValid _returnvalue_2
    (:Is%20Valid
      (Utilities|IsValid _returnvalue_3
        (:Is%20Valid
          (CallFunction|KillLastEnemyCamShake MeshComp)
          (Game|Damage|ApplyDamage _returnvalue_3 1.0 0 _returnvalue "/Script/Engine.DamageType")
          (Class|BPIPlayer|IncreaseCombo(Message) _returnvalue)
          (return true))))))

(fn KillLastEnemyCamShake
  (params (MeshComp :type Skeletal%20Mesh%20Component%20Object%20Reference))
  (bind _returnvalue (Components|GetOwner MeshComp))
  (bind _returnvalue_2 (Actor|GetComponentbyClass _returnvalue "/Game/FFCS/Blueprints/AC_FFCC.AC_FFCC_C"))
  (bind _returnvalue_3 (Components|GetOwner MeshComp))
  (bind _returnvalue_4 (Actor|GetComponentbyClass _returnvalue_3 "/Game/FFCS/Blueprints/AC_AIDirector.AC_AIDirector_C"))
  (bind _returnvalue_5 (Class|FreeFlowCombatComponent|GetCurrentEnemy _returnvalue_2))
  (bind _returnvalue_6 (Class|FreeFlowCombatComponent|GetCounterEnemy _returnvalue_2))
  (if (GameplayTags|MatchesAnyTags (Class|FreeFlowCombatComponent|GetTag _returnvalue_2) (GameplayTags|MakeLiteralGameplayTagContainer "(GameplayTags=((TagName=\"PlayerStates.Combat\"),(TagName=\"PlayerStates.CombatInProgress\")))") true)
    (Utilities|IsValid _returnvalue_5
      (:Is%20Valid
        (if (== (Variables|/Script/FFCS.CharacterBase|GetCurrentHealth (.AsCharacter%20Base (Utilities|Casting|CastToCharacterBase _returnvalue_5))) 1.0)
          (Utilities|IsValid _returnvalue_4 :!label _label
            (:Is%20Valid
              (if (== (Utilities|Array|Length (Variables|/Game/FFCS/Blueprints/AC_AIDirector.AC_AIDirector_C|GetEnemies _returnvalue_4)) 1)
                (CameraShakes|StartCameraShake (Game|GetPlayerCameraManager 0) "/Game/FFCS/Blueprints/BP_CameraShake.BP_CameraShake_C" 1.0 "World" "0, 0, 0")
                (return true)))))))
    (else
      (Utilities|IsValid _returnvalue_6
        (:Is%20Valid
          (if (== (Variables|/Script/FFCS.CharacterBase|GetCurrentHealth (.AsCharacter%20Base (Utilities|Casting|CastToCharacterBase _returnvalue_6))) 1.0)
            (goto _label)))))))