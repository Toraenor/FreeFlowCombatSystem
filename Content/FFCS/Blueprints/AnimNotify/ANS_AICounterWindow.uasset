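; Anim notify state that marks an AI counter window in enemy animations by toggling a counter indicator.
; On begin it casts the mesh owner to BP_Enemy and shows its CounterIcon component; on end it hides the icon again.
; It changes only the icon's visibility and does nothing for owners that are not BP_Enemy.
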(fn ReceivedNotifyBegin
  (params (MeshComp :type Skeletal%20Mesh%20Component%20Object%20Reference) (Animation :type Anim%20Sequence%20Base%20Object%20Reference) (TotalDuration :type Float%20%28single-precision%29) (EventReference :type Anim%20Notify%20Event%20Reference%20Structure%20%28by%20ref%29))
  (bind _asbp_enemy (Utilities|Casting|CastToBP_Enemy (Components|GetOwner MeshComp)))
  (Rendering|SetVisibility (Variables|/Game/FFCS/Blueprints/BP_Enemy.BP_Enemy_C|GetCounterIcon _asbp_enemy) true false)
  (return true))

(fn ReceivedNotifyEnd
  (params (MeshComp :type Skeletal%20Mesh%20Component%20Object%20Reference) (Animation :type Anim%20Sequence%20Base%20Object%20Reference) (EventReference :type Anim%20Notify%20Event%20Reference%20Structure%20%28by%20ref%29))
  (bind _asbp_enemy (Utilities|Casting|CastToBP_Enemy (Components|GetOwner MeshComp)))
  (Rendering|SetVisibility (Variables|/Game/FFCS/Blueprints/BP_Enemy.BP_Enemy_C|GetCounterIcon _asbp_enemy) false false)
  (return true))