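; Anim notify state that keeps an AI character's motion warp target up to date during an animation.
; Each tick, it gets a teleport location and rotation from the owner's AC_EnemyComp using an Offset, then writes them to the "Target" warp target on its MotionWarpingComponent.
; The update runs only when both components are valid on the owner.
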(fn ReceivedNotifyTick
  (params (MeshComp :type Skeletal%20Mesh%20Component%20Object%20Reference) (Animation :type Anim%20Sequence%20Base%20Object%20Reference) (FrameDeltaTime :type Float%20%28single-precision%29) (EventReference :type Anim%20Notify%20Event%20Reference%20Structure%20%28by%20ref%29))
  (bind _returnvalue (Components|GetOwner MeshComp))
  (bind _returnvalue_2 (Actor|GetComponentbyClass _returnvalue "/Game/FFCS/Blueprints/AC_EnemyComp.AC_EnemyComp_C"))
  (bind _returnvalue_3 (Actor|GetComponentbyClass _returnvalue "/Script/MotionWarping.MotionWarpingComponent"))
  (if (and (Utilities|IsValid _returnvalue_2) (Utilities|IsValid _returnvalue_3))
    (bind (_location _rotation) (Default|GetEnemyTeleportLocation _returnvalue_2 (Variables|Default|GetOffset)))
    (Class|MotionWarpingComponent|AddorUpdateWarpTargetfromLocationandRotation _returnvalue_3 "Target" _location _rotation)
    (return true)))