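; AN_KillCameraShake is an animation notify that shakes the player camera during an attack animation, apparently to accent a killing blow.
; It gets the current enemy from the mesh owner's AC_FFCC component and casts it to CharacterBase.
; BP_CameraShake plays in world space on player 0's camera manager only when that enemy is valid and its CurrentHealth equals exactly 1.0.
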(fn ReceivedNotify
  (params (MeshComp :type Skeletal%20Mesh%20Component%20Object%20Reference) (Animation :type Anim%20Sequence%20Base%20Object%20Reference) (EventReference :type Anim%20Notify%20Event%20Reference%20Structure%20%28by%20ref%29))
  (bind _returnvalue (Components|GetOwner MeshComp))
  (bind _returnvalue_2 (Actor|GetComponentbyClass _returnvalue "/Game/FFCS/Blueprints/AC_FFCC.AC_FFCC_C"))
  (bind _returnvalue_3 (Class|FreeFlowCombatComponent|GetCurrentEnemy _returnvalue_2))
  (Utilities|IsValid _returnvalue_3
    (:Is%20Valid
      (if (== (Variables|/Script/FFCS.CharacterBase|GetCurrentHealth (.AsCharacter%20Base (Utilities|Casting|CastToCharacterBase _returnvalue_3))) 1.0)
        (CameraShakes|StartCameraShake (Game|GetPlayerCameraManager 0) "/Game/FFCS/Blueprints/BP_CameraShake.BP_CameraShake_C" 1.0 "World" "0, 0, 0")
        (return true)
        (else
          (return true))))
    (:Is%20Not%20Valid
      (return true))))