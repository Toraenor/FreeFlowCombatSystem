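; Anim notify state that slows an enemy's active montage over the notify window, apparently for counter animations.
; On begin, it sets the montage play rate to SlowPlayRate only if the owner has an AC_EnemyComp whose IsInCounterAnimPart is false.
; On end, it restores the play rate to 1 unconditionally.
; It changes montage speed only, as a global time dilation reset is left unconnected.
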(fn ReceivedNotifyBegin
  (params (MeshComp :type Skeletal%20Mesh%20Component%20Object%20Reference) (Animation :type Anim%20Sequence%20Base%20Object%20Reference) (TotalDuration :type Float%20%28single-precision%29) (EventReference :type Anim%20Notify%20Event%20Reference%20Structure%20%28by%20ref%29))
  (bind _returnvalue (Components|SkeletalMesh|GetAnimInstance MeshComp))
  (bind _returnvalue_2 (Components|GetOwner MeshComp))
  (bind _returnvalue_3 (Actor|GetComponentbyClass _returnvalue_2 "/Game/FFCS/Blueprints/AC_EnemyComp.AC_EnemyComp_C"))
  (Utilities|IsValid _returnvalue_3
    (:Is%20Valid
      (if (not (Variables|/Game/FFCS/Blueprints/AC_EnemyComp.AC_EnemyComp_C|GetIsInCounterAnimPart _returnvalue_3))
        (Animation|Montage|MontageSetPlayRate _returnvalue (Animation|Montage|GetCurrentActiveMontage _returnvalue) (Variables|Default|GetSlowPlayRate))
        (return true)))))

(fn ReceivedNotifyEnd
  (params (MeshComp :type Skeletal%20Mesh%20Component%20Object%20Reference) (Animation :type Anim%20Sequence%20Base%20Object%20Reference) (EventReference :type Anim%20Notify%20Event%20Reference%20Structure%20%28by%20ref%29))
  (bind _returnvalue (Components|SkeletalMesh|GetAnimInstance MeshComp))
  (Animation|Montage|MontageSetPlayRate _returnvalue (Animation|Montage|GetCurrentActiveMontage _returnvalue) 1.0)
  (return true))