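; AN_AIPlayerCounterAnimPart is an animation notify in FFCS, named for the AI and player counter animation.
; It finds the owner's AC_FFCC component and validates its counter enemy and that enemy's AC_EnemyComp.
; The checks lead to no action.
; An unconnected ApplyDamage node targeting the counter enemy never runs, so the notify currently has no gameplay effect.
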(fn ReceivedNotify
  (params (MeshComp :type Skeletal%20Mesh%20Component%20Object%20Reference) (Animation :type Anim%20Sequence%20Base%20Object%20Reference) (EventReference :type Anim%20Notify%20Event%20Reference%20Structure%20%28by%20ref%29))
  (bind _returnvalue (Components|GetOwner MeshComp))
  (bind _returnvalue_2 (Actor|GetComponentbyClass _returnvalue "/Game/FFCS/Blueprints/AC_FFCC.AC_FFCC_C"))
  (bind _returnvalue_3 (Class|FreeFlowCombatComponent|GetCounterEnemy _returnvalue_2))
  (Utilities|IsValid _returnvalue_2
    (:Is%20Valid
      (LocalVariables|SetFFCC _returnvalue_2)
      (Utilities|IsValid _returnvalue_3
        (:Is%20Valid
          (Utilities|IsValid (Actor|GetComponentbyClass _returnvalue_3 "/Game/FFCS/Blueprints/AC_EnemyComp.AC_EnemyComp_C")))))))