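; Player combat component that tracks the current and counter enemies and a gameplay-tag player state, and runs counter attacks.
; Counters start the enemy-supplied player montage at the enemy montage's normalized progress and trigger the enemy's counter animation.
; Montage completion or interruption resets to Idle, applies damage, and restores camera mode and time dilation if needed.
; Helpers pick random close/mid/long-range attacks, classify hit direction by yaw, and check teleport distance.
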(event EventPlayCounterMontage
  (bind _returnvalue (CallFunction|GetCounterEnemy))
  (bind _returnvalue_2 (Actor|GetComponentbyClass _returnvalue "/Game/FFCS/Blueprints/AC_EnemyComp.AC_EnemyComp_C"))
  (bind _playercountermontage (Variables|/Game/FFCS/Blueprints/AC_EnemyComp.AC_EnemyComp_C|GetPlayerCounterMontage _returnvalue_2))
  (Utilities|IsValid _returnvalue
    (:Is%20Valid
      (Utilities|IsValid _returnvalue_2
        (:Is%20Valid
          (Utilities|IsValid _playercountermontage
            (:Is%20Valid
              (bind _ascharacter (Utilities|Casting|CastToCharacter (CallFunction|GetCounterEnemy)))
              (Utilities|IsValid (Animation|Montage|GetCurrentActiveMontage (Components|SkeletalMesh|GetAnimInstance (Variables|/Script/Engine.Character|GetMesh _ascharacter)))
                (:Is%20Valid
                  (Animation|Montage|PlayMontage (Actor|GetComponentbyClass (Components|GetOwner) "/Script/Engine.SkeletalMeshComponent") _playercountermontage 1.0 (* (/ (Animation|Montage|MontageGetPosition (Components|SkeletalMesh|GetAnimInstance (Variables|/Script/Engine.Character|GetMesh _ascharacter)) (Animation|Montage|GetCurrentActiveMontage (Components|SkeletalMesh|GetAnimInstance (Variables|/Script/Engine.Character|GetMesh _ascharacter)))) (Animation|GetPlayLength (Animation|Montage|GetCurrentActiveMontage (Components|SkeletalMesh|GetAnimInstance (Variables|/Script/Engine.Character|GetMesh _ascharacter))))) (Animation|GetPlayLength _playercountermontage))
                    (:then
                      (bind _asbp_enemy (Utilities|Casting|CastToBP_Enemy (CallFunction|GetCounterEnemy)))
                      (Default|PlayCounterAnim _asbp_enemy (Animation|Montage|MontageGetPosition (Components|SkeletalMesh|GetAnimInstance (Variables|/Script/Engine.Character|GetMesh _ascharacter)) (Animation|Montage|GetCurrentActiveMontage (Components|SkeletalMesh|GetAnimInstance (Variables|/Script/Engine.Character|GetMesh _ascharacter))))))
                    (:OnCompleted
                      (CallFunction|SetTagtoPlayer "(TagName=\"PlayerStates.Idle\")" :!label _label)
                      (Game|Damage|ApplyDamage _asbp_enemy 1.0 0 (Components|GetOwner) "/Script/Engine.DamageType")
                      (bind _asbp_player (Utilities|Casting|CastToBP_Player (Components|GetOwner)))
                      (if (Utilities|Enum|NotEqual(Enum) (Variables|/Game/FFCS/Blueprints/BP_Player.BP_Player_C|GetCurrentCameraMode _asbp_player) "NewEnumerator0")
                        (Default|InterpolateCameraMode _asbp_player "NewEnumerator0")
                        (Utilities|Time|SetGlobalTimeDilation 1.0)))
                    (:OnInterrupted
                      (goto _label))))
                (:Is%20Not%20Valid
                  (goto _label))))))))))

(fn GetMontageBasedonDistance
  (bind _returnvalue (CallFunction|GetCurrentEnemy))
  (bind _returnvalue_2 (Components|GetOwner))
  (bind _distances (Variables|Default|GetDistances))
  (bind _returnvalue_3 (Transformation|GetActorLocation _returnvalue))
  (bind _returnvalue_4 (Transformation|GetActorLocation _returnvalue_2))
  (bind _output (Utilities|Array|Get(acopy) _distances))
  (bind _returnvalue_5 (Math|Vector|Distance(Vector) _returnvalue_3 _returnvalue_4))
  (if (Math|Float|InRange(Float) _returnvalue_5 0.0 _output true false)
    (bind _out_row (CallFunction|GetRandomAnimfromDT "/Game/FFCS/Data/DT_CloseRangeAttacks.DT_CloseRangeAttacks"))
    (return _out_row)
    (elif (Math|Float|InRange(Float) _returnvalue_5 _output (Utilities|Array|Get(acopy) _distances 1))
      (bind _out_row_2 (CallFunction|GetRandomAnimfromDT "/Game/FFCS/Data/DT_MidRangeAttacks.DT_MidRangeAttacks"))
      (return _out_row_2)
      (else
        (bind _out_row_3 (CallFunction|GetRandomAnimfromDT "/Game/FFCS/Data/DT_LongRangeAttacks.DT_LongRangeAttacks"))
        (return _out_row_3)))))

(fn HitDirection
  (params (Instigator :type Actor%20Object%20Reference))
  (bind _returnvalue (Transformation|GetActorLocation Instigator))
  (bind _returnvalue_2 (Components|GetOwner))
  (bind _returnvalue_3 (Transformation|GetActorRotation _returnvalue_2))
  (bind _returnvalue_4 (Transformation|GetActorLocation _returnvalue_2))
  (bind _returnvalue_5 (Math|Rotator|FindLookatRotation _returnvalue_4 _returnvalue))
  (bind _returnvalue_6 (Math|Rotator|Delta(Rotator) _returnvalue_5 _returnvalue_3))
  ;[1 0.1521 0.8232] Checking from direction enemy has been hit, in order :
  ; Forward
  ; Right
  ; Backward
  ; Left
  (if (Math|Float|InRange(Float) (.yaw _returnvalue_6) -45.0 45.0)
    (return "Fwd")
    (elif (Math|Float|InRange(Float) (.yaw _returnvalue_6) 45.0 135.0)
      (return "Right")
      (elif (or (Math|Float|InRange(Float) (.yaw _returnvalue_6) 135.0 1.8e+02) (Math|Float|InRange(Float) (.yaw _returnvalue_6) -179.99 -135.0))
        (return "Backward")
        (else
          (return "Left"))))))

(fn GetCurrentEnemy
  (return (Variables|Default|GetCurrentEnemy)))

(fn SetCurrentEnemy
  (params (Enemy :type Actor%20Object%20Reference))
  (bind _output_get (Variables|Default|SetCurrentEnemy Enemy))
  (Utilities|IsValid _output_get
    (:Is%20Valid
      (Utilities|IsValid (Actor|GetComponentbyClass _output_get "/Game/FFCS/Blueprints/AC_EnemyComp.AC_EnemyComp_C")
        (:Is%20Valid
          (Default|ControlEnemyLogic (Actor|GetComponentbyClass _output_get "/Game/FFCS/Blueprints/AC_EnemyComp.AC_EnemyComp_C") true))))))

(fn GetTag
  (return (Variables|Default|GetPlayerStateTag)))

(fn SetTagtoPlayer
  (params (Tag :type Gameplay%20Tag%20Structure))
  (bind _output_get (Variables|Default|SetPlayerStateTag Tag))
  (Development|PrintString (Utilities|String|ToString(Name) (GameplayTags|GetTagName _output_get))))

(fn SetCounterEnemy
  (params (Enemy :type Actor%20Object%20Reference))
  (Variables|Default|SetCounterEnemy Enemy))

(fn GetCounterEnemy
  (return (Variables|Default|GetCounterEnemy)))

(fn CheckDistancefromCounterEnemy
  (return (> (Transformation|GetDistanceTo (Variables|Default|GetCounterEnemy) (Components|GetOwner)) (Variables|Default|GetTeleportDistance))))