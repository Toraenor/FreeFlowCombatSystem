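; Enemy character that reacts to hits and tracks the player through AI perception.
; Damage plays a directional hit montage via ACEnemyComp and calls ApplyDamages; when the montage ends, a still-targetable enemy resets its component logic after a short delay.
; Sensing the player registers it with the player's AC_AIDirector and sets the TargetActor blackboard key.
; Losing perception starts a grace timer, cancelled on re-sensing, that unregisters it and clears the key.
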(event OnTargetPerceptionUpdated(AIPerception)
  (params (Actor :type Actor%20Object%20Reference) (Stimulus :type AI%20Stimulus%20Structure))
  (bind _returnvalue (Actor|GetComponentbyClass Actor "/Game/FFCS/Blueprints/AC_AIDirector.AC_AIDirector_C"))
  (if (Variables|Default|GetTargetable)
    (if (== Actor (Game|GetPlayerCharacter 0))
      (if (.bSuccessfullySensed (Utilities|Struct|BreakAIStimulus Stimulus))
        (Development|PrintString (Utilities|String|Append (Utilities|String|MakeLiteralString "Sensed ") (Utilities|GetDisplayName Actor)))
        (Utilities|Time|ClearandInvalidateTimerbyHandle (Variables|Default|GetTargetCheckerTimerHandle))
        (Utilities|IsValid _returnvalue
          (:Is%20Valid
            (Default|AddEnemy _returnvalue self))
          (:Is%20Not%20Valid
            _))
        (AI|Components|Blackboard|SetValueasObject (AI|GetBlackboard 0) (Utilities|Name|MakeLiteralName "TargetActor") Actor)
        (else
          (bind _returnvalue_2 (Utilities|Time|SetTimerbyEvent (delegate Custom|LostPlayer) 2.0))
          (Variables|Default|SetTargetCheckerTimerHandle _returnvalue_2))))))

(event Custom|ResetEnemyLogicToNormal
  (bind _ac_enemycomp (Variables|Default|GetAC_EnemyComp))
  (Utilities|IsValid _ac_enemycomp
    (:Is%20Valid
      (Default|ControlEnemyLogic _ac_enemycomp false))))

(event Custom|LostPlayer
  (bind _returnvalue (Utilities|Name|MakeLiteralName "TargetActor"))
  (bind _returnvalue_2 (AI|GetBlackboard 0))
  (bind _returnvalue_3 (Utilities|Name|MakeLiteralName "TargetActor"))
  (bind _returnvalue_4 (AI|GetBlackboard 0))
  (bind _returnvalue_5 (AI|Components|Blackboard|GetValueasObject _returnvalue_2 _returnvalue_3))
  (bind _returnvalue_6 (AI|Components|Blackboard|GetValueasObject _returnvalue_4 _returnvalue))
  (bind _ascharacter (Utilities|Casting|CastToCharacter _returnvalue_5))
  (bind _returnvalue_7 (Actor|GetComponentbyClass _ascharacter "/Game/FFCS/Blueprints/AC_AIDirector.AC_AIDirector_C"))
  (Utilities|IsValid _returnvalue_6
    (:Is%20Valid
      (Development|PrintString (Utilities|String|Append (Utilities|String|MakeLiteralString "Lost ") (Utilities|GetDisplayName _returnvalue_6)))
      (Utilities|IsValid _returnvalue_5
        (:Is%20Valid
          (Utilities|IsValid _returnvalue_7
            (:Is%20Valid
              (Default|RemoveEnemy _returnvalue_7 self))
            (:Is%20Not%20Valid
              _))
          (AI|Components|Blackboard|SetValueasObject (AI|GetBlackboard 0) (Utilities|Name|MakeLiteralName "TargetActor") 0))))))

(event EventBeginPlay
  (|CallParentFunction))

(event Game|Damage|EventAnyDamage
  (params (Damage :type Float%20%28single-precision%29) (DamageType :type Damage%20Type%20Object%20Reference) (InstigatedBy :type Controller%20Object%20Reference) (DamageCauser :type Actor%20Object%20Reference))
  (bind _ac_enemycomp (Variables|Default|GetAC_EnemyComp))
  (bind _returnvalue (Class|EnemyComponent|HitDirection _ac_enemycomp DamageCauser))
  (Animation|Montage|PlayMontage (Variables|Character|GetMesh) (Utilities|Select :Index _returnvalue :Fwd "/Game/FFCS/Animations/AnimMontages/Hit/AM_HitForward.AM_HitForward" :Right "/Game/FFCS/Animations/AnimMontages/Hit/AM_HitRight.AM_HitRight" :Backward "/Game/FFCS/Animations/AnimMontages/Hit/AM_HitBack.AM_HitBack" :Left "/Game/FFCS/Animations/AnimMontages/Hit/AM_HitLeft.AM_HitLeft")
    (:then
      (Class|CharacterBase|ApplyDamages Damage _returnvalue))
    (:OnCompleted
      (if (Variables|Default|GetTargetable) :!label _label
        (Utilities|Time|SetTimerbyEvent (delegate Custom|ResetEnemyLogicToNormal) 1.0)))
    (:OnBlendOut
      (goto _label))
    (:OnInterrupted
      (goto _label))))

(fn ConstructionScript
  (|CallParentFunction))